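; Trigger-volume actor that repeatedly plays a sound at random points around itself or the player while the player is inside.
; Construction script adds a sphere, capsule or box trigger by shape setting.
; Overlap or player-spawn check starts a looping timer, its random interval picked once per start; leaving clears it.
; Each tick offsets the sound into the upper hemisphere within a range and spawns a BP_testActor at a similarly randomized point.
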(event `self.ReceiveBeginPlay`
  (bind _asbp_first_person_character (cast `/Game/FirstPerson/Blueprints/BP_FirstPersonCharacter` (`GameplayStatics.GetPlayerPawn` 0)))
  (add `/Game/FirstPerson/Blueprints/BP_FirstPersonCharacter.PlayerSpawn` _asbp_first_person_character (`|CreateDelegate` :!event `verifOnPlayerSpawn`)))

(event `verifOnPlayerSpawn`
  (for _ (`self.GetOverlappingActors` "/Game/FirstPerson/Blueprints/BP_FirstPersonCharacter.BP_FirstPersonCharacter_C")
    (`KismetSystemLibrary.K2_SetTimer` null "playsound" (`KismetMathLibrary.RandomFloatInRange` (`self.MinTimeBetweenSounds`) (`self.MaxTimeBetweenSounds`)) true :!label _label)))

(event `BeginOverlap`
  (params (OverlappedComponent :type "PrimitiveComponent Object Reference") (OtherActor :type "Actor Object Reference") (OtherComp :type "PrimitiveComponent Object Reference") (OtherBodyIndex :type Integer) (bFromSweep :type Boolean) (SweepResult :type "HitResult Structure (by ref)"))
  (cast `/Game/FirstPerson/Blueprints/BP_FirstPersonCharacter` OtherActor)
  (goto _label))

(event `EndOverlap`
  (params (OverlappedComponent :type "PrimitiveComponent Object Reference") (OtherActor :type "Actor Object Reference") (OtherComp :type "PrimitiveComponent Object Reference") (OtherBodyIndex :type Integer))
  (cast `/Game/FirstPerson/Blueprints/BP_FirstPersonCharacter` OtherActor)
  (`KismetSystemLibrary.K2_ClearTimer` null "playsound"))

(event `playsound`
  (bind (_returnvalue_x _returnvalue_y _returnvalue_z) (`KismetMathLibrary.BreakVector` (`KismetMathLibrary.RandomUnitVector`)))
  (bind _returnvalue (+ (`self.K2_GetActorLocation` (select `bool` (`self.FromThePlayer?`) :`false` self :`true` (`GameplayStatics.GetPlayerPawn` 0) :!type "Actor Object Reference")) (* (`KismetMathLibrary.MakeVector` _returnvalue_x _returnvalue_y (`KismetMathLibrary.Sqrt` (`KismetMathLibrary.Square` _returnvalue_z))) (`KismetMathLibrary.RandomFloatInRange` (`self.MinRangeFromTarget`) (`self.MaxRangeFromTarget`)))))
  (`GameplayStatics.PlaySoundAtLocation` (`self.SoundToPlay`) _returnvalue (struct) (`self.VolumeMultiplier`) 1.0 0.0 null null null null)
  (`|SpawnActorFromClass` "/Game/BP_testActor.BP_testActor_C" (`KismetMathLibrary.MakeTransform` _returnvalue) "Undefined" "MultiplyWithRoot" null null))

(fn `UserConstructionScript`
  (switch `/Game/ETypeOfShape` (`self.TypeOfShape`)
    (:`NewEnumerator0`
      (bind _returnvalue (`AddComponent|NODE_AddSphereComponent-0`))
      (add `PrimitiveComponent.OnComponentBeginOverlap` _returnvalue (`|CreateDelegate` :!event `BeginOverlap`))
      (add `PrimitiveComponent.OnComponentEndOverlap` _returnvalue (`|CreateDelegate` :!event `EndOverlap`)))
    (:`NewEnumerator1`
      (bind _returnvalue_2 (`AddComponent|NODE_AddCapsuleComponent-0`))
      (add `PrimitiveComponent.OnComponentBeginOverlap` _returnvalue_2 (`|CreateDelegate` :!event `BeginOverlap`))
      (add `PrimitiveComponent.OnComponentEndOverlap` _returnvalue_2 (`|CreateDelegate` :!event `EndOverlap`)))
    (:`NewEnumerator2`
      (bind _returnvalue_3 (`AddComponent|NODE_AddBoxComponent-0`))
      (add `PrimitiveComponent.OnComponentBeginOverlap` _returnvalue_3 (`|CreateDelegate` :!event `BeginOverlap`))
      (add `PrimitiveComponent.OnComponentEndOverlap` _returnvalue_3 (`|CreateDelegate` :!event `EndOverlap`)))))